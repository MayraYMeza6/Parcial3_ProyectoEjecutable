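; BP_Jugador is the player character, moving along the world X axis and losing lives to threats.
; Tick polls A and D for movement, Space jumps, and a debug key binding on S crouches.
; Hitting a BP_Amenaza removes one of the lives set on BeginPlay, prints the remainder and destroys the threat.
; When no lives remain, it opens MapaPrincipal.
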(event EventBeginPlay
  (Variables|Default|SetVidas%20 5)
  (Pawn|Components|CharacterMovement|SetMovementMode (Variables|Character|GetCharacterMovement) "MOVE_Walking" 2))

(event Collision|EventActorBeginOverlap
  (params (OtherActor :type Actor%20Object%20Reference)))

(event EventTick
  (params (DeltaSeconds :type Float%20%28single-precision%29))
  (bind _returnvalue (Game|GetPlayerController 0))
  (if (Game|Player|IsInputKeyDown _returnvalue "D")
    (Pawn|Input|AddMovementInput "1.000000,0.000000,0.000000" 1.0 false)
    (elif (Game|Player|IsInputKeyDown _returnvalue "A")
      (Pawn|Input|AddMovementInput "1.000000,0.000000,0.000000" -1.0 false))))

(event Collision|EventHit
  (params (MyComp :type Primitive%20Component%20Object%20Reference) (Other :type Actor%20Object%20Reference) (OtherComp :type Primitive%20Component%20Object%20Reference) (bSelfMoved :type Boolean) (HitLocation :type Vector :default "0, 0, 0") (HitNormal :type Vector :default "0, 0, 0") (NormalImpulse :type Vector :default "0, 0, 0") (Hit :type Hit%20Result%20Structure%20%28by%20ref%29))
  (bind _asbp_amenaza (Utilities|Casting|CastToBP_Amenaza Other))
  (bind _output_get (Variables|Default|SetVidas%20 (- (Variables|Default|GetVidas%20) 1)))
  (Development|PrintString (Utilities|String|ToString(Integer) _output_get) true true "(R=0.590625,G=0.111095,B=0.000000,A=1.000000)")
  (Actor|DestroyActor _asbp_amenaza)
  (if (not (> (Variables|Default|GetVidas%20) 0))
    (Game|OpenLevel(byName) "MapaPrincipal")))

(event Input|KeyboardEvents|DebugKeyS
  (params (Key :type Key%20Structure :default "None") (ActionValue :type Input%20Action%20Value%20Structure))
  ;[0.15 0.15 0.15 0.5] Agacharse
  (:Pressed
    (Character|Crouch))
  (:Released
    (Character|UnCrouch)))

(event Input|KeyboardEvents|SpaceBar
  (params (Key :type Key%20Structure :default "None"))
  ;[0.15 0.15 0.15 0.5] Saltar
  (:Pressed
    (Character|Jump))
  (:Released
    (Character|StopJumping)))

(fn ConstructionScript)